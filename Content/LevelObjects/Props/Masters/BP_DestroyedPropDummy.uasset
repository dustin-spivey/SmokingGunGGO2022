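; Dummy actor for a destroyed, frozen prop that breaks with Chaos, then melts away and removes itself.
; The construction script creates one dynamic instance of the frozen freezeable-object material and applies it to every material slot on DestroyedProp.
; The first Chaos break event, gated by DoOnce, waits briefly, then plays the Melt timeline to drive that material's Opacity before destroying the actor.
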(event OnChaosBreakEvent(DestroyedProp)
  (params (BreakEvent :type Chaos%20Break%20Event%20Structure%20%28by%20ref%29))
  (Utilities|FlowControl|DoOnce false
    (:Completed
      (Utilities|FlowControl|Delay 2.5)
      (bind _opacity (Timeline|Melt Play)
        (:Update
          (Rendering|Material|SetScalarParameterValue (Variables|Default|GetDynamicMaterial) "Opacity" _opacity :!class /Script/Engine.MaterialInstanceDynamic))
        (:Finished
          (Actor|DestroyActor))))))

(event EventBeginPlay)

(event Collision|EventActorBeginOverlap
  (params (OtherActor :type Actor%20Object%20Reference)))

(event EventTick
  (params (DeltaSeconds :type Float%20%28single-precision%29)))

(fn ConstructionScript
  (bind _destroyedprop (Variables|Default|GetDestroyedProp))
  (bind _returnvalue (Rendering|Material|CreateDynamicMaterialInstance "/Game/LevelObjects/Props/Masters/Materials/MI_FreezeableObjectMaster_Frozen.MI_FreezeableObjectMaster_Frozen" "None" "None" :!class /Script/Engine.KismetMaterialLibrary))
  (Variables|Default|SetDynamicMaterial _returnvalue)
  (for (_ _array_index) (Rendering|Material|GetMaterials _destroyedprop)
    (Rendering|Material|SetMaterial _destroyedprop _array_index (Variables|Default|GetDynamicMaterial))))