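; Master freezeable prop that ices over when hit by a SnowBall, then shatters when a SnowBall overlaps it once iced.
; A dynamic material instance receives the local-space hit location, and the Ice timeline grows an ice radius from it at a size-scaled play rate.
; When the timeline finishes, the prop counts as Iced, so the next Box overlap spawns DestroyedPropActor at the mesh transform and destroys this actor.
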(event OnComponentHit(SM_DestructibleCube)
  (params (HitComponent :type Primitive%20Component%20Object%20Reference) (OtherActor :type Actor%20Object%20Reference) (OtherComp :type Primitive%20Component%20Object%20Reference) (NormalImpulse :type Vector :default "0, 0, 0") (Hit :type Hit%20Result%20Structure%20%28by%20ref%29))
  (Utilities|Casting|CastToSnowBall OtherActor)
  (if (not (Variables|Default|GetIced))
    (Utilities|FlowControl|DoOnce false
      (:Completed
        (Rendering|Material|SetVectorParameterValue (Variables|Default|GetMaterial) "HitLocation" (Math|Conversions|ToLinearColor(Vector) (Math|Transform|InverseTransformLocation (Transformation|GetActorTransform) (.Location (Collision|BreakHitResult Hit)))) :!class /Script/Engine.MaterialInstanceDynamic)
        (CallFunction|IceOver)))))

(event OnComponentBeginOverlap(Box)
  (params (OverlappedComponent :type Primitive%20Component%20Object%20Reference) (OtherActor :type Actor%20Object%20Reference) (OtherComp :type Primitive%20Component%20Object%20Reference) (OtherBodyIndex :type Integer) (bFromSweep :type Boolean) (SweepResult :type Hit%20Result%20Structure%20%28by%20ref%29))
  (Utilities|Casting|CastToSnowBall OtherActor)
  (if (Variables|Default|GetIced)
    (Utilities|FlowControl|DoOnce false
      (:Completed
        (Game|SpawnActorfromClass (Variables|Default|GetDestroyedPropActor) (Transformation|GetWorldTransform (Variables|Default|GetSM_DestructibleCube)) "Undefined" 0 0)
        (Actor|DestroyActor)))))

(event Custom|IceOver
  (Components|Timeline|SetPlayRate (Variables|Default|GetIce) (/ 5e+02 (Variables|Default|GetIceTransitionRadiusSize)))
  (bind _iceamount (Timeline|Ice PlayFromStart)
    (:Update
      (Rendering|Material|SetScalarParameterValue (Variables|Default|GetMaterial) "IceRadius" (* _iceamount (Variables|Default|GetIceTransitionRadiusSize)) :!class /Script/Engine.MaterialInstanceDynamic))
    (:Finished
      (Variables|Default|SetIced true))))

(event EventBeginPlay
  (Physics|SetSimulatePhysics (Variables|Default|GetSM_DestructibleCube) (Variables|Default|GetSimulatePhysics)))

(fn ConstructionScript
  (bind _returnvalue (Rendering|Material|CreateDynamicMaterialInstance (Variables|Default|GetParentMaterial) "None" "None" :!class /Script/Engine.KismetMaterialLibrary))
  (bind _output_get (Variables|Default|SetMaterial _returnvalue))
  (Rendering|Material|SetMaterial (Variables|Default|GetSM_DestructibleCube) 0 _output_get))